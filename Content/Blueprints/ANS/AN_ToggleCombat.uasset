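; AN_ToggleCombat is an animation notify that switches the owning character between combat and non-combat states during an animation.
; It finds the owner's CMP_Combat component and, if a main weapon is valid, reattaches it to its hand socket or stowed attach socket based on the EnableCombat flag.
; It then sets the component's combat-enabled state to match, and returns false when no weapon exists.
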(fn ReceivedNotify
  (params (MeshComp :type Skeletal%20Mesh%20Component%20Object%20Reference) (Animation :type Anim%20Sequence%20Base%20Object%20Reference) (EventReference :type Anim%20Notify%20Event%20Reference%20Structure%20%28by%20ref%29))
  (bind _returnvalue (Components|GetOwner MeshComp))
  (bind _returnvalue_2 (Actor|GetComponentbyClass _returnvalue "/Game/Blueprints/CMP/CMP_Combat.CMP_Combat_C"))
  (bind _mainweapon (Default|GetMainWeapon _returnvalue_2))
  (Utilities|IsValid _mainweapon
    (:Is%20Valid
      (Default|AttachActor _mainweapon (select (Variables|Default|GetEnableCombat) (Variables|/Game/Blueprints/Combat/Weapon/BP_Equipable_Base.BP_Equipable_Base_C|GetHandSocketName _mainweapon) (Variables|/Game/Blueprints/Combat/Weapon/BP_Equipable_Base.BP_Equipable_Base_C|GetAttach%20Socket%20Name _mainweapon)))
      (Default|SetIsCombatEnabled _returnvalue_2 (Variables|Default|GetEnableCombat))
      (return true))
    (:Is%20Not%20Valid
      (return false))))