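; Combat component that holds a character's main weapon, combat-enabled state and attack combo state.
; It picks montages and stamina cost by action type from a data table, by index or at random, falling back to the main weapon's lookup.
; Weapon swaps unequip and destroy an actor, and combat toggles notify the anim instance through an interface.
; GetActionCost is an empty stub.
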(fn GetMontagesbyAction
  (params (ActionType :type E_MontageAction%20Enum :default "NewEnumerator0") (Idx :type Integer) (RandomIdx :type Boolean))
  (bind (_returnvalue _mainweapon) (CallFunction|GetMainWeapon))
  (bind _returnvalue_2 (Utilities|String|EnumtoString ActionType))
  (bind (_success _montages _stamaniacost) (Default|GetMontagesbyAction _mainweapon ActionType Idx RandomIdx))
  (Development|PrintString _returnvalue_2)
  (bind _returnvalue_3 (Utilities|GetDataTableRow (Variables|Default|GetMontageDataTable) (Utilities|String|StringToName _returnvalue_2))
    (:then
      (return true (select RandomIdx (.OutItem (Utilities|Array|Random (.Montages (Utilities|Struct|BreakSt_MontageAction _returnvalue_3)))) (select (Utilities|Array|IsValidIndex (.Montages (Utilities|Struct|BreakSt_MontageAction _returnvalue_3)) Idx) (Utilities|Array|Get(acopy) (.Montages (Utilities|Struct|BreakSt_MontageAction _returnvalue_3)) Idx) (Utilities|Array|Get(acopy) (.Montages (Utilities|Struct|BreakSt_MontageAction _returnvalue_3))))) (.StamaniaCost (Utilities|Struct|BreakSt_MontageAction _returnvalue_3))))
    (:RowNotFound
      (if _returnvalue
        (return _success _montages _stamaniacost)
        (else
          (return false 0 0.0))))))

(fn ResetAttack
  (Variables|Default|SetbIsAttackSaved false)
  (Variables|Default|SetAttackCount 0)
  (Variables|Default|SetAttackType "NewEnumerator1"))

(fn SetMainWeapon
  (params (MainWeapon :type BP%20Weapon%20Base%20Object%20Reference))
  (Utilities|FlowControl|Sequence
    (:then_0
      (Utilities|IsValid (Variables|Default|GetMainWeapon)
        (:Is%20Valid
          (Default|OnUnEquipped (Variables|Default|GetMainWeapon))
          (Actor|DestroyActor (Variables|Default|GetMainWeapon)))))
    (:then_1
      (Variables|Default|SetMainWeapon MainWeapon))))

(fn GetMainWeapon
  (bind _mainweapon (Variables|Default|GetMainWeapon))
  (return (Utilities|IsValid _mainweapon) _mainweapon))

(fn SetIsCombatEnabled
  (params (bIsCombatEnabled :type Boolean))
  (bind _output_get (Variables|Default|SetbIsCombatEnabled bIsCombatEnabled))
  (Class|BPIAnimInstance|BPIAnimUpdateCombatEnabled(Message) (Components|SkeletalMesh|GetAnimInstance (Variables|/Script/Engine.Character|GetMesh (.AsCharacter (Utilities|Casting|CastToCharacter (Components|GetOwner))))) _output_get))

(fn GetIsCombatEnabled
  (return (Variables|Default|GetbIsCombatEnabled)))

(fn SetAttackType
  (params (AttackType :type E_MontageAction%20Enum :default "NewEnumerator0"))
  (Variables|Default|SetAttackType AttackType))

(fn GetAttackType
  (return (Variables|Default|GetAttackType)))

(fn IncreaseAttackCount
  (bind _result (Math|Integer|IncrementInt (Variables|Default|GetAttackCount))
    (:%20%20
      (if (not (.Success (CallFunction|GetMontagesbyAction (Variables|Default|GetAttackType) _result false)))
        (Variables|Default|SetAttackCount 0)))))

(fn GetAttackCount
  (return (Variables|Default|GetAttackCount)))

(fn GetActionCost)