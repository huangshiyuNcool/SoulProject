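; Collision hit component that detects hits along a mesh, between two sockets, while collision is activated.
; Each Tick it runs a multi sphere trace for objects from the start socket to the end socket, skipping ignored actors.
; New actors are recorded and broadcast through OnHit, so each is reported once until activation clears the list.
; Functions set the traced mesh, manage the ignore list and expose hit state.
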(event Custom|ActivateCollision
  (CallFunction|ClearHitActors)
  (Variables|Default|SetbIsCollisionEnabled true))

(event Custom|DeActivateCollsion
  (Variables|Default|SetbIsCollisionEnabled false))

(event Custom|ClearHitActors
  (Utilities|Array|Clear (Variables|Default|GetAlreadyHitActors)))

(event Custom|CollisionTrace
  (bind (_outhits _returnvalue) (Collision|MultiSphereTraceForObjects (Transformation|GetSocketLocation (Variables|Default|GetCollisionMeshComponent) (Variables|Initialization|GetStartSocket)) (Transformation|GetSocketLocation (Variables|Default|GetCollisionMeshComponent) (Variables|Initialization|GetEndSocket)) (Variables|Initialization|GetRadius) (Variables|Default|GetCollisionObject%20Types) false (Variables|Default|GetActors%20to%20Ignore) (Variables|Initialization|GetDraw%20Debug%20Type)))
  (if _returnvalue
    (for _array_element _outhits
      (bind _output_get (Variables|Default|SetlastHit _array_element))
      (if (not (Utilities|Array|ContainsItem (Variables|Default|GetAlreadyHitActors) (.HitActor (Collision|BreakHitResult _output_get))))
        (bind _output_get_2 (Variables|Default|SetHitActor (.HitActor (Collision|BreakHitResult _output_get))))
        (Utilities|Array|Add (Variables|Default|GetAlreadyHitActors) _output_get_2)
        (Default|CallOnHit (Variables|Default|GetlastHit))))))

(event EventTick
  (params (DeltaSeconds :type Float%20%28single-precision%29))
  (if (Variables|Default|GetbIsCollisionEnabled)
    (CallFunction|CollisionTrace)))

(fn GetAlreadyHitActors
  (return (Variables|Default|GetAlreadyHitActors)))

(fn GetIsCollisionEnabled
  (return (Variables|Default|GetbIsCollisionEnabled)))

(fn GetLastHit
  (return (Variables|Default|GetlastHit)))

(fn GetCollsionMeshComponent
  (return (Variables|Default|GetCollisionMeshComponent)))

(fn SetCollisionMeshComponent
  (params (CollisionMeshComponent :type Primitive%20Component%20Object%20Reference))
  (Variables|Default|SetCollisionMeshComponent CollisionMeshComponent))

(fn AddActorIgnore
  (params (NewItem :type Actor%20Object%20Reference%20%28by%20ref%29))
  (Utilities|Array|AddUnique (Variables|Default|GetActors%20to%20Ignore) NewItem))

(fn RemoveActorIgnore
  (params (Item :type Actor%20Object%20Reference%20%28by%20ref%29))
  (Utilities|Array|RemoveItem (Variables|Default|GetActors%20to%20Ignore) Item))

(fn GetActorstoIgnore
  (return (Variables|Default|GetActors%20to%20Ignore)))