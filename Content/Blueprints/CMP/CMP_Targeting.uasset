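; Actor component that gives its owning Character a toggleable lock-on targeting mode.
; Enabling sphere-traces forward for configured object types, stores the hit actor and switches movement rotation to orient to camera.
; While locked, Tick interpolates the control rotation's pitch and yaw toward the target, preserving roll.
; Disabling clears the target and restores the default rotation mode.
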(event Custom|EnableLockOn
  (bind (_find _foundtraget) (CallFunction|FindTarget))
  (if _find
    (CallFunction|SetLockTarget _foundtraget)
    (CallFunction|SetIsTargeting true)
    (CallFunction|SetRotationMode "NewEnumerator0")))

(event Custom|DisableLockOn
  (CallFunction|SetIsTargeting false)
  (CallFunction|SetLockTarget)
  (CallFunction|SetRotationMode (Variables|Default|GetDefaultRotationMode)))

(event Custom|ToggleLockOn
  (if (not (CallFunction|GetIsTargeting))
    (CallFunction|EnableLockon)
    (else
      (CallFunction|DisableLockon))))

(event EventBeginPlay
  (bind _ascharacter (Utilities|Casting|CastToCharacter (Components|GetOwner)))
  (bind _output_get (Variables|Default|SetOwnerCharacter _ascharacter))
  (Variables|Default|SetOwnerController (Pawn|GetController _output_get))
  (Variables|Default|SetFollowCamera (Actor|GetComponentbyClass (Variables|Default|GetOwnerCharacter) "/Script/Engine.CameraComponent")))

(event EventTick
  (params (DeltaSeconds :type Float%20%28single-precision%29))
  (if (CallFunction|GetIsTargeting)
    (CallFunction|UpdateTargetingControllerRotation)))

(fn SetIsTargeting
  (params (IsTargeting :type Boolean))
  (Variables|Default|SetbIsTargeting IsTargeting))

(fn GetIsTargeting
  (return (Variables|Default|GetbIsTargeting)))

(fn FindTarget
  (bind _returnvalue (Components|GetOwner))
  (bind _returnvalue_2 (Transformation|GetActorLocation _returnvalue))
  (bind (_outhit _returnvalue_3) (Collision|SphereTraceForObjects _returnvalue_2 (+ _returnvalue_2 (* (Transformation|GetActorForwardVector (Variables|Default|GetOwnerCharacter)) (Variables|Initialization|GetTargetingDistance))) (Variables|Initialization|GetTargetingRaius) (Variables|Initialization|GetTargetingObjectTypes) false (Utilities|Array|MakeArray (Components|GetOwner)) "None"))
  (if (and _returnvalue_3 (Utilities|IsValid (.HitActor (Collision|BreakHitResult _outhit))))
    (return true (.HitActor (Collision|BreakHitResult _outhit)))
    (else
      (return false 0))))

(fn SetLockTarget
  (params (TragetActor :type Actor%20Object%20Reference))
  (Variables|Default|SetTragetActor TragetActor))

(fn UpdateTargetingControllerRotation
  (bind _returnvalue (Components|GetOwner))
  (bind _returnvalue_2 (Utilities|Time|GetWorldDeltaSeconds))
  (bind _tragetactor (Variables|Default|GetTragetActor))
  (bind _interp_speed (Variables|Default|GetInterp%20Speed))
  (bind _ownercontroller (Variables|Default|GetOwnerController))
  (bind _returnvalue_3 (Transformation|GetActorRotation _ownercontroller))
  (bind _returnvalue_4 (Transformation|GetActorLocation _returnvalue))
  (bind _returnvalue_5 (Transformation|GetActorLocation _tragetactor))
  (bind _returnvalue_6 (Math|Rotator|FindLookatRotation _returnvalue_4 _returnvalue_5))
  (bind _returnvalue_7 (Math|Interpolation|RInterpTo _returnvalue_3 _returnvalue_6 _returnvalue_2 _interp_speed))
  (if (and (Utilities|IsValid (Variables|Default|GetOwnerController)) (Utilities|IsValid (Variables|Default|GetTragetActor)))
    (Pawn|SetControlRotation (Variables|Default|GetOwnerController) (Math|Rotator|MakeRotator (.Roll (Math|Rotator|BreakRotator _returnvalue_3)) (.pitch _returnvalue_7) (.yaw _returnvalue_7)))))

(fn SetRotationMode
  (params (RotationMode :type E_RotationMode%20Enum :default "NewEnumerator0"))
  (bind _ownercharacter (Variables|Default|GetOwnerCharacter))
  (bind _charactermovement (Variables|/Script/Engine.Character|GetCharacterMovement _ownercharacter))
  (bind _output_get (Variables|Default|SetCurrentRotationMode RotationMode))
  (switch Utilities|FlowControl|Switch|SwitchonE_RotationMode _output_get
    (:NewEnumerator0
      (Variables|/Script/Engine.Pawn|SetbUseControllerRotationYaw _ownercharacter false)
      (Variables|/Script/Engine.CharacterMovementComponent|SetbUseControllerDesiredRotation _charactermovement true)
      (Variables|/Script/Engine.CharacterMovementComponent|SetbOrientRotationToMovement _charactermovement false))
    (:NewEnumerator1
      (Variables|/Script/Engine.Pawn|SetbUseControllerRotationYaw _ownercharacter false)
      (Variables|/Script/Engine.CharacterMovementComponent|SetbUseControllerDesiredRotation _charactermovement false)
      (Variables|/Script/Engine.CharacterMovementComponent|SetbOrientRotationToMovement _charactermovement true))))

(fn GetRotationMode
  (return (Variables|Default|GetCurrentRotationMode)))