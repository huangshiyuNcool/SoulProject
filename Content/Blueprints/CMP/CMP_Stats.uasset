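; Actor component that holds a character's stats, such as HP and stamina, as base, max and current values in maps.
; Current-value changes go through a setter that notifies listeners, with clamping on modification.
; Damage lowers HP, sets one of two states on CMP_CharacterStateManager and returns whether HP reached zero.
; Looping timers regenerate stamina; HP regen has no implementation, and stamina drain is not started here.
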(event Custom|StartRegen
  (params (Stat :type E_Stats%20Enum :default "NewEnumerator0"))
  (switch Utilities|FlowControl|Switch|SwitchonE_Stats Stat
    (:NewEnumerator2
      (Utilities|Time|SetTimerbyFunctionName 0 "RegenStamina" 0.1 true))))

(event Custom|StopRegen
  (params (Stat :type E_Stats%20Enum :default "NewEnumerator0"))
  (switch Utilities|FlowControl|Switch|SwitchonE_Stats Stat
    (:NewEnumerator2
      (Utilities|Time|ClearTimerbyFunctionName 0 "RegenStamina"))))

(event EventBeginPlay
  (CallFunction|StartRegen "NewEnumerator0"))

(event EventTick
  (params (DeltaSeconds :type Float%20%28single-precision%29)))

(fn SetCurrentStatValue
  (params (KeyStat :type E_Stats%20Enum :default "NewEnumerator0") (Value :type Float%20%28double-precision%29))
  (Utilities|Map|Add (Variables|BaseStats|GetCurrentStats) KeyStat Value)
  (Default|CallOnCurrentStatValueUpted KeyStat Value))

(fn GetCurrentStatValue
  (params (KeyStat :type E_Stats%20Enum :default "NewEnumerator0"))
  (return (.Value (Utilities|Map|Find (Variables|BaseStats|GetCurrentStats) KeyStat))))

(fn InitializeStats
  (bind _basestats (Variables|BaseStats|GetBaseStats))
  (bind _keys (Utilities|Map|Keys _basestats))
  (for _array_element _keys
    (CallFunction|SetCurrentStatValue _array_element (.BaseValue (Utilities|Struct|BreakSt_BaseStat (.Value (Utilities|Map|Find _basestats _array_element)))))))

(fn ModifyCurrentStatValue
  (params (Stat :type E_Stats%20Enum :default "NewEnumerator0") (Value :type Float%20%28double-precision%29) (ShouldRegen :type Boolean))
  (if (!= Value 0.0)
    (CallFunction|StopRegen Stat)
    (bind _output_get (LocalVariables|SetLValue (+ (CallFunction|GetCurrentStatValue Stat) Value)))
    (CallFunction|SetCurrentStatValue Stat (Math|Float|Clamp(Float) _output_get 0.0 (BaseStats|GetMaxStatValue Stat)))
    (if ShouldRegen
      (CallFunction|StartRegen Stat))))

(fn GetBaseStatValue
  (params (KeyStat :type E_Stats%20Enum :default "NewEnumerator0"))
  (return (.BaseValue (Utilities|Struct|BreakSt_BaseStat (.Value (Utilities|Map|Find (Variables|BaseStats|GetBaseStats) KeyStat))))))

(fn GetMaxStatValue
  (params (KeyStat :type E_Stats%20Enum :default "NewEnumerator0"))
  (return (.MaxValue (Utilities|Struct|BreakSt_BaseStat (.Value (Utilities|Map|Find (Variables|BaseStats|GetBaseStats) KeyStat))))))

(fn SetBaseStatValue
  (params (KeyStat :type E_Stats%20Enum :default "NewEnumerator0") (Value :type Float%20%28double-precision%29))
  (bind _basestats (Variables|BaseStats|GetBaseStats))
  (bind _structout (Utilities|Struct|SetmembersinSt_BaseStat (.Value (Utilities|Map|Find _basestats KeyStat)) Value))
  (Utilities|Map|Add _basestats KeyStat _structout))

(fn SetMaxStatValue
  (params (KeyStat :type E_Stats%20Enum :default "NewEnumerator0") (Value :type Float%20%28double-precision%29))
  (bind _basestats (Variables|BaseStats|GetBaseStats))
  (bind _structout (Utilities|Struct|SetmembersinSt_BaseStat (.Value (Utilities|Map|Find _basestats KeyStat)) Value))
  (Utilities|Map|Add _basestats KeyStat _structout))

(fn TakeDamge
  (params (InDamage :type Float%20%28double-precision%29))
  (CallFunction|ModifyCurrentStatValue "NewEnumerator0" (* InDamage -1.0) false)
  (if (<= (CallFunction|GetCurrentStatValue "NewEnumerator0") 0.0)
    (Default|SetState (Actor|GetComponentbyClass (Components|GetOwner) "/Game/Blueprints/CMP/CMP_CharacterStateManager.CMP_CharacterStateManager_C") "NewEnumerator4")
    (return true)
    (else
      (Default|SetState (Actor|GetComponentbyClass (Components|GetOwner) "/Game/Blueprints/CMP/CMP_CharacterStateManager.CMP_CharacterStateManager_C") "NewEnumerator5")
      (return false))))

(fn RegenStamina
  (bind _value (CallFunction|GetCurrentStatValue "NewEnumerator2"))
  (bind _maxvalue (BaseStats|GetMaxStatValue "NewEnumerator2"))
  (CallFunction|SetCurrentStatValue "NewEnumerator2" (Math|Float|Clamp(Float) (+ (CallFunction|GetCurrentStatValue "NewEnumerator2") (Variables|StatRegen|GetStaminaRegenRate)) 0.0 (BaseStats|GetMaxStatValue "NewEnumerator2")))
  (Development|PrintString (Utilities|String|Append (Utilities|String|ToString(Float) _value) "//" (Utilities|String|ToString(Float) _maxvalue)))
  (if (>= _value _maxvalue)
    (Utilities|Time|ClearTimerbyFunctionName 0 "RegenStamina")))

(fn ConsumeStamina
  (CallFunction|SetCurrentStatValue "NewEnumerator2" (Math|Float|Clamp(Float) (- (CallFunction|GetCurrentStatValue "NewEnumerator2") (Variables|StatRegen|GetStaminaConsumeRate)) 0.0 (BaseStats|GetMaxStatValue "NewEnumerator2")))
  (if (<= (CallFunction|GetCurrentStatValue "NewEnumerator2") 0.0)
    (Utilities|Time|ClearTimerbyFunctionName 0 "ConsumeStamina")))