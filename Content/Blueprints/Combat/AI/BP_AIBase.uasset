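; Base AI combat character that can be targeted, showing lock-on and health widgets while targeted.
; State manager tags trigger dodge, death, disable and combat-toggle actions, playing montages from the combat component, while the stats component handles health and stamina, including timer-driven sprint drain.
; Point damage applies stats loss, AI hearing report and impact effects; death ragdolls body and weapon.
; Attack logic exists but is never called, and hit reaction is an empty stub.
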(event OnStateBegin(CMP_CharacterStateManager)
  (params (CharacterState :type Gameplay%20Tag%20Structure))
  (|SwitchGameplayTag CharacterState
    (:Character.State.Doging
      (CallFunction|PerformDoge))
    (:Character.State.Dead
      (CallFunction|PerformDeath))
    (:Character.State.Disabled
      (CallFunction|PerformDisabled))
    (:Character.State.Toggling
      (CallFunction|PerformToggleCombat))))

(event OnStateEnd(CMP_CharacterStateManager)
  (params (CharacterState :type Gameplay%20Tag%20Structure))
  (|SwitchGameplayTag CharacterState
    (:Character.State.Attacking
      (Default|ResetAttack (Variables|Default|GetCMP_Combat)))))

(event OnCharacterActionBegin(CMP_CharacterStateManager)
  (params (NewAction :type Gameplay%20Tag%20Structure)))

(event OnCharacterActionEnd(CMP_CharacterStateManager)
  (params (EndAction :type Gameplay%20Tag%20Structure)))

(event Custom|ApplyHitReaction
  (params (DamageType :type E_DamageType%20Enum :default "NewEnumerator0"))
  (switch Utilities|FlowControl|Switch|SwitchonE_DamageType DamageType))

(event EventBPICombatResetCombat
  ;[1 1 1] 状态恢复
  (if (not (Default|IsCurrentStateEqualtoArray (Variables|Default|GetCMP_CharacterStateManager) "(GameplayTags=((TagName=\"Character.State.Dead\")))"))
    (Default|SetState (Variables|Default|GetCMP_CharacterStateManager) "(TagName=\"Character.State.None\")")
    (Default|StartRegen (Variables|Default|GetCMP_Stats) "NewEnumerator2")))

(event EventBeginPlay
  ;[1 1 1] BeginPlay
  (Default|Init (Variables|Default|GetCMP_CharacterStateManager))
  (Default|InitializeStats (Variables|Default|GetCMP_Stats))
  (CallFunction|SetSpeedMode "NewEnumerator1")
  (bind _returnvalue (UserInterface|CreateWidget "/Game/Blueprints/UI/UMG_Health.UMG_Health_C" 0 (Variables|Default|GetCMP_Stats) false))
  (UserInterface|SetWidget (Variables|Default|GetWidget_Health) _returnvalue))

(event Game|Damage|EventPointDamage
  (params (Damage :type Float%20%28single-precision%29) (DamageType :type Damage%20Type%20Object%20Reference) (HitLocation :type Vector :default "0, 0, 0") (HitNormal :type Vector :default "0, 0, 0") (HitComponent :type Primitive%20Component%20Object%20Reference) (BoneName :type Name :default "None") (ShotFromDirection :type Vector :default "0, 0, 0") (InstigatedBy :type Controller%20Object%20Reference) (DamageCauser :type Actor%20Object%20Reference) (HitInfo :type Hit%20Result%20Structure%20%28by%20ref%29))
  ;[1 1 1] 受到伤害
  (bind _asbp_attack_damage_type (Utilities|Casting|CastToBP_AttackDamageType DamageType))
  (if (CallFunction|CanTakeDamge)
    (Default|TakeDamge (Variables|Default|GetCMP_Stats) Damage)
    (Class|AISenseDamage|ReportDamageEvent self (Pawn|GetControlledPawn InstigatedBy) Damage HitLocation HitLocation "None")
    (CallFunction|DamageEffect HitInfo)
    (CallFunction|ApplyHitReaction (Variables|/Game/Blueprints/DamageType/BP_AttackDamageType.BP_AttackDamageType_C|GetDamageType _asbp_attack_damage_type))))

(event EventBPITargetonTargeted
  (params (bIsTargeted :type Boolean))
  ;[1 1 1] 被锁定显示UI
  (Rendering|SetVisibility (Variables|Default|GetWidget_Lock) bIsTargeted false))

(event Input|ActionEvents|InputActionDoge
  (params (Key :type Key%20Structure :default "None"))
  ;[1 1 1] 闪避行为
  (:Pressed
    (if (CallFunction|CanPerformDoge)
      (Default|SetState (Variables|Default|GetCMP_CharacterStateManager) "(TagName=\"Character.State.Doging\")"))))

(fn ConstructionScript)

(fn PerformMontageAction
  (params (ActionType :type Gameplay%20Tag%20Structure :default "(TagName=\"Character.Action.None\")") (Idx :type Integer) (RandomIdx :type Boolean) (StartSectionName :type Name))
  (bind _cmp_combat (Variables|Default|GetCMP_Combat))
  (bind (_success _montages _stamaniacost) (Default|GetMontagesbyAction _cmp_combat ActionType Idx RandomIdx))
  (bind _output_get (LocalVariables|SetTmpMontage _montages))
  (Utilities|IsValid _output_get
    (:Is%20Valid
      (Animation|PlayAnimMontage (LocalVariables|GetTmpMontage) 1.0 StartSectionName)
      (Default|SetCurrentAction (Variables|Default|GetCMP_CharacterStateManager) ActionType))
    (:Is%20Not%20Valid
      _))
  (return _success _stamaniacost))

(fn CanPerformJump
  (return (Default|IsCurrentStateEqualtoArray (Variables|Default|GetCMP_CharacterStateManager) (GameplayTags|MakeGameplayTagContainerfromTag "(TagName=\"Character.State.None\")"))))

(fn CanPerformToggleCombat
  (return (and (Utilities|IsValid (.MainWeapon (Default|GetMainWeapon (Variables|Default|GetCMP_Combat)))) (Default|IsCurrentStateEqualtoArray (Variables|Default|GetCMP_CharacterStateManager) "(GameplayTags=((TagName=\"Character.State.None\")))"))))

(fn PerformToggleCombat
  (CallFunction|PerformMontageAction (select (Default|GetIsCombatEnabled (Variables|Default|GetCMP_Combat)) "(TagName=\"Character.Action.ExitCombat\")" "(TagName=\"Character.Action.EnterCombat\")") 0 false "None"))

(fn CanPerformAttack
  (bind _cmp_stats (Variables|Default|GetCMP_Stats))
  (bind _cmp_characterstatemanager (Variables|Default|GetCMP_CharacterStateManager))
  (return (Math|Boolean|ANDBoolean (or (Default|IsCurrentStateEqualtoArray _cmp_characterstatemanager "(GameplayTags=((TagName=\"Character.State.None\")))") (and (Default|IsCurrentStateEqualtoArray _cmp_characterstatemanager "(GameplayTags=((TagName=\"Character.State.Attacking\")))") (Variables|/Game/Blueprints/CMP/CMP_Combat.CMP_Combat_C|GetbIsAttackSaved (Variables|Default|GetCMP_Combat)))) (Default|GetIsCombatEnabled (Variables|Default|GetCMP_Combat)) (> (Default|GetCurrentStatValue _cmp_stats "NewEnumerator2") (Variables|/Game/Blueprints/CMP/CMP_Stats.CMP_Stats_C|GetLimitStamania _cmp_stats)))))

(fn PerformAttack
  (bind _cmp_combat (Variables|Default|GetCMP_Combat))
  (bind _cmp_combat_2 (Variables|Default|GetCMP_Combat))
  (if (AI|Components|NavMovement|IsFalling (Variables|Character|GetCharacterMovement))
    (Default|SetAttackType (Variables|Default|GetCMP_Combat) "(TagName=\"Character.Action.Attack.ChargeAttack\")")
    (elif (and (Utilities|Enum|Equal(Enum) (Variables|Default|GetSpeedMode) "NewEnumerator2") (> (Math|Vector|VectorLength (Variables|/Script/Engine.MovementComponent|GetVelocity (Variables|Character|GetCharacterMovement))) 0.0))
      (Default|SetAttackType (Variables|Default|GetCMP_Combat) "(TagName=\"Character.Action.Attack.SprintAttack\")")))
  (bind _stamaniacost (CallFunction|PerformMontageAction (Default|GetAttackType _cmp_combat) (Default|GetAttackCount _cmp_combat) false (select (Variables|/Game/Blueprints/CMP/CMP_Combat.CMP_Combat_C|GetbIsAttackSaved _cmp_combat) "Start" "None")))
  (Variables|/Game/Blueprints/CMP/CMP_Combat.CMP_Combat_C|SetbIsAttackSaved _cmp_combat_2 false)
  (Default|IncreaseAttackCount _cmp_combat_2)
  (Default|ModifyCurrentStatValue (Variables|Default|GetCMP_Stats) "NewEnumerator2" (* _stamaniacost -1.0) false))

(fn CanPerformDoge
  (bind _cmp_stats (Variables|Default|GetCMP_Stats))
  (return (Math|Boolean|ANDBoolean (.Success (Default|GetMontagesbyAction (Variables|Default|GetCMP_Combat) "(TagName=\"Character.Action.Doge\")" 0 false)) (Default|IsCurrentStateEqualtoArray (Variables|Default|GetCMP_CharacterStateManager) "(GameplayTags=((TagName=\"Character.State.None\"),(TagName=\"Character.State.Attacking\")))") (> (Default|GetCurrentStatValue _cmp_stats "NewEnumerator2") (Variables|/Game/Blueprints/CMP/CMP_Stats.CMP_Stats_C|GetLimitStamania _cmp_stats)))))

(fn PerformDoge
  (bind _stamaniacost (CallFunction|PerformMontageAction "(TagName=\"Character.Action.Doge\")" 0 false "None"))
  (Default|ModifyCurrentStatValue (Variables|Default|GetCMP_Stats) "NewEnumerator2" (* _stamaniacost -1.0) false))

(fn CanTakeDamge
  (return (not (Default|IsCurrentStateEqualtoArray (Variables|Default|GetCMP_CharacterStateManager) "(GameplayTags=((TagName=\"Character.State.Dead\")))"))))

(fn PerformDisabled
  (if (not (Default|IsCurrentStateEqualtoArray (Variables|Default|GetCMP_CharacterStateManager) "(GameplayTags=((TagName=\"Character.State.Dead\"),(TagName=\"Character.State.Attacking\")))"))
    (CallFunction|PerformMontageAction "(TagName=\"Character.Action.Disable\")" 0 false "None")))

(fn PerformDeath
  (bind _mesh (Variables|Character|GetMesh))
  (bind _cmp_combat (Variables|Default|GetCMP_Combat))
  (bind _pelvisbonename (Variables|Default|GetPelvisBoneName))
  (bind _mainweapon (Default|GetMainWeapon _cmp_combat))
  (Pawn|Components|CharacterMovement|SetMovementMode (Variables|Character|GetCharacterMovement) "MOVE_None" 0)
  (Collision|SetCollisionEnabled (Variables|Collision|GetCapsuleComponent) "NoCollision")
  (Collision|SetCollisionProfileName (Variables|Character|GetMesh) "PhysicsActor" true :!class /Script/Engine.PrimitiveComponent)
  (Class|SkeletalMeshComponent|SetAllBodiesBelowSimulatePhysics _mesh _pelvisbonename true true)
  (Class|SkeletalMeshComponent|SetAllBodiesBelowPhysicsBlendWeight _mesh _pelvisbonename 1.0 false true)
  (CallFunction|ApplyHitReactionPhysicsVelocity 2e+03)
  (Utilities|IsValid _mainweapon
    (:Is%20Valid
      (Default|CESimulatePhysics _mainweapon))))

(fn ApplyHitReactionPhysicsVelocity
  (params (InitialSpeed :type Float%20%28double-precision%29))
  (Physics|SetPhysicsLinearVelocity (Variables|Character|GetMesh) (* (Transformation|GetActorForwardVector) (* InitialSpeed -1.0)) false "None"))

(fn SetSpeedMode
  (params (SpeedMode :type E_SpeedMode%20Enum :default "NewEnumerator0"))
  (bind _output_get (Variables|Default|SetSpeedMode SpeedMode))
  (Default|UpdateRotaionMode (Variables|Default|GetCMP_Targeting))
  (if (Utilities|Enum|Equal(Enum) _output_get "NewEnumerator2")
    (Utilities|Time|SetTimerbyFunctionName 0 "MoveStaminaCost" 0.1 true)
    (else
      (Utilities|Time|ClearTimerbyFunctionName 0 "MoveStaminaCost")
      (Default|StartRegen (Variables|Default|GetCMP_Stats) "NewEnumerator2")
      (Variables|/Script/Engine.CharacterMovementComponent|SetMaxWalkSpeed (Variables|Character|GetCharacterMovement) (.Value (Utilities|Map|Find (Variables|Default|GetSpeedValue) (Variables|Default|GetSpeedMode))))
      (Variables|Default|SetConsumed false))))

(fn DamageEffect
  (params (HitInfo :type Hit%20Result%20Structure))
  (bind _location (Collision|BreakHitResult HitInfo))
  (Audio|PlaySoundatLocation "/Game/SoundFX/Gruntling/A_Guardian_Impact01_Cue.A_Guardian_Impact01_Cue" _location "0, 0, 0" 1.0 1.0 0.0 0 0 0 0)
  (Effects|SpawnEmitteratLocation "/Game/StarterContent/Particles/P_Explosion.P_Explosion" _location))

(fn CanSprint
  (return (and (> (Default|GetCurrentStatValue (Variables|Default|GetCMP_Stats) "NewEnumerator2") 0.0) (not (Variables|Default|GetConsumed)))))

(fn MoveStaminaCost
  (bind _cmp_stats (Variables|Default|GetCMP_Stats))
  (if (CallFunction|CanSprint)
    (if (> (Math|Vector|VectorLength (Variables|/Script/Engine.MovementComponent|GetVelocity (Variables|Character|GetCharacterMovement))) 0.0)
      (Default|ModifyCurrentStatValue (Variables|Default|GetCMP_Stats) "NewEnumerator2" -2.0 true)
      (Variables|/Script/Engine.CharacterMovementComponent|SetMaxWalkSpeed (Variables|Character|GetCharacterMovement) (.Value (Utilities|Map|Find (Variables|Default|GetSpeedValue) "NewEnumerator2"))))
    (else
      (Variables|Default|SetConsumed true)
      (Variables|/Script/Engine.CharacterMovementComponent|SetMaxWalkSpeed (Variables|Character|GetCharacterMovement) (.Value (Utilities|Map|Find (Variables|Default|GetSpeedValue) "NewEnumerator1")))
      (if true
        (Variables|Default|SetConsumed (<= (Default|GetCurrentStatValue _cmp_stats "NewEnumerator2") (* (Default|GetMaxStatValue _cmp_stats "NewEnumerator2") 0.5)))))))

(fn BPICombatGetDesireRotation
  (if (Utilities|Operators|NotEqual(!=) :A (Pawn|Components|PawnMovement|GetLastInputVector (Variables|Character|GetCharacterMovement)) :ErrorTolerance 0.001)
    (return (Math|Conversions|RotationFromXVector (Class|Pawn|GetLastMovementInputVector)))
    (else
      (return (Transformation|GetActorRotation)))))

(fn BPICombatGetSpeedMode
  (return (Variables|Default|GetSpeedMode)))

(fn BPITargetCanbeTargeted
  (return (not (Default|IsCurrentStateEqualtoArray (Variables|Default|GetCMP_CharacterStateManager) "(GameplayTags=((TagName=\"Character.State.Dead\")))"))))