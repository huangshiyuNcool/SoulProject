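; BP_WeaponDual is a dual-wield weapon that extends its parent weapon with a second, left-hand mesh copied from the main mesh.
; On equip and combat toggle, the left mesh attaches to either its hand or stowed socket on the owning character.
; A separate left collision component ignores the owner and applies point damage on hit, while ActivateCollision and DeActivateCollision route to the main or left component by weapon part.
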(event OnHit(CMP_CollisionHit_L)
  (params (HitResult :type Hit%20Result%20Structure))
  (Game|Damage|ApplyPointDamage (.HitActor (Collision|BreakHitResult HitResult)) (Variables|Default|GetBase%20Damage) (Transformation|GetActorForwardVector (Components|GetOwner)) HitResult (Game|GetInstigatorController) self))

(event EventBeginPlay
  (|CallParentFunction) ; This node is disabled and will not be called.\nDrag off pins to build functionality.
)

(event Collision|EventActorBeginOverlap
  (params (OtherActor :type Actor%20Object%20Reference))
  (|CallParentFunction OtherActor) ; This node is disabled and will not be called.\nDrag off pins to build functionality.
)

(event EventTick
  (params (DeltaSeconds :type Float%20%28single-precision%29))
  (|CallParentFunction DeltaSeconds) ; This node is disabled and will not be called.\nDrag off pins to build functionality.
)

(event EventToggleCombat
  (params (bIsCombatEnabled :type Boolean))
  (|CallParentFunction bIsCombatEnabled)
  (ItemMesh|AttachMeshL (select bIsCombatEnabled (Variables|Default|GetHandSocketName_L) (Variables|Default|GetAttachSocketName_L))))

(fn ConstructionScript
  (|CallParentFunction)
  (Components|StaticMesh|SetStaticMesh (Variables|Default|GetStaticMesh_L) (Variables|/Script/Engine.StaticMeshComponent|GetStaticMesh (Variables|Default|GetStaticMesh))))

(fn OnEquipped
  (bind _cmp_collisionhit_l (Variables|Default|GetCMP_CollisionHit_L))
  (|CallParentFunction)
  (Default|SetCollisionMeshComponent (Variables|Default|GetCMP_CollisionHit_L) (Variables|Default|GetStaticMesh_L))
  (ItemMesh|AttachMeshL (select (Default|GetIsCombatEnabled (Variables|Default|GetCMPCombat)) (Variables|Default|GetHandSocketName_L) (Variables|Default|GetAttachSocketName_L)))
  (Default|SetCollisionMeshComponent _cmp_collisionhit_l (Variables|Default|GetStaticMesh_L))
  (Default|AddActorIgnore _cmp_collisionhit_l (Components|GetOwner)))

(fn AttachActor
  (params (SocketName :type Name :default "None"))
  (|CallParentFunction SocketName))

(fn ActivateCollision
  (params (WeaponPart :type E_WeaponPart%20Enum :default "NewEnumerator0"))
  (switch Utilities|FlowControl|Switch|SwitchonE_WeaponPart WeaponPart
    (:NewEnumerator0
      (Default|ActivateCollision (Variables|Default|GetCMP_CollisionHit_Main)))
    (:NewEnumerator1
      (Default|ActivateCollision (Variables|Default|GetCMP_CollisionHit_L)))))

(fn DeActivateCollision
  (params (WeaponPart :type E_WeaponPart%20Enum :default "NewEnumerator0"))
  (switch Utilities|FlowControl|Switch|SwitchonE_WeaponPart WeaponPart
    (:NewEnumerator0
      (Default|DeActivateCollsion (Variables|Default|GetCMP_CollisionHit_Main)))
    (:NewEnumerator1
      (Default|DeActivateCollsion (Variables|Default|GetCMP_CollisionHit_L)))))

(fn AttachMeshL
  (params (SocketName :type Name))
  (Transformation|AttachComponentToComponent (Variables|Default|GetStaticMesh_L) (Variables|/Script/Engine.Character|GetMesh (.AsCharacter (Utilities|Casting|CastToCharacter (Components|GetOwner)))) SocketName "SnapToTarget" "SnapToTarget" "SnapToTarget" true))