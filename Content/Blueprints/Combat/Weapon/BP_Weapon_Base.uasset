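; BP_Weapon_Base is the base weapon that handles equipping, hit damage and action montage lookup.
; On equip it attaches to a hand or holster socket by combat state, registers with CMP_Combat, sends its combat type to the AnimInstance and configures CMP_CollisionHit.
; Collision hits apply point damage, and an event switches the mesh to physics simulation.
; Montages and stamina costs come from a DataTable keyed by action enum, picked by index or randomly.
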(event OnHit(CMP_CollisionHit)
  (params (HitResult :type Hit%20Result%20Structure))
  (Game|Damage|ApplyPointDamage (.HitActor (Collision|BreakHitResult HitResult)) (Variables|Default|GetBase%20Damage) (Transformation|GetActorForwardVector (Components|GetOwner)) HitResult (Game|GetInstigatorController) self))

(event Custom|CE_SimulatePhysics
  (bind _mesh (CallFunction|GetItemMesh))
  (Collision|SetCollisionProfileName _mesh "PhysicsActor" true :!class /Script/Engine.PrimitiveComponent)
  (Physics|SetSimulatePhysics _mesh true))

(fn ConstructionScript
  (|CallParentFunction))

(fn OnEquipped
  (bind _cmp_collisionhit (Variables|Default|GetCMP_CollisionHit))
  (CallFunction|SetIsEquipped true)
  (Variables|Default|SetCMPCombat (Actor|GetComponentbyClass (Components|GetOwner) "/Game/Blueprints/CMP/CMP_Combat.CMP_Combat_C"))
  (CallFunction|AttachActor (select (Default|GetIsCombatEnabled (Variables|Default|GetCMPCombat)) (Variables|Default|GetHandSocketName) (Variables|Default|GetAttach%20Socket%20Name)))
  (Default|SetMainWeapon (Variables|Default|GetCMPCombat) self)
  (Class|BPIAnimInstance|BPIAnimUpdateCombatType(Message) (Components|SkeletalMesh|GetAnimInstance (Variables|/Script/Engine.Character|GetMesh (.AsCharacter (Utilities|Casting|CastToCharacter (Components|GetOwner))))) (Variables|Default|GetCombatType))
  (Default|SetCollisionMeshComponent _cmp_collisionhit (CallFunction|GetItemMesh))
  (Default|AddActorIgnore _cmp_collisionhit (Components|GetOwner)))

(fn GetMontagesbyAction
  (params (ActionType :type E_MontageAction%20Enum :default "NewEnumerator0") (Idx :type Integer) (RandomIdx :type Boolean))
  (bind _returnvalue (Utilities|GetDataTableRow (Variables|Default|GetMontageDataTable) (Utilities|String|StringToName (Utilities|String|EnumtoString ActionType)))
    (:then
      (return true (select RandomIdx (.OutItem (Utilities|Array|Random (.Montages (Utilities|Struct|BreakSt_MontageAction _returnvalue)))) (Utilities|Array|Get(acopy) (.Montages (Utilities|Struct|BreakSt_MontageAction _returnvalue)) Idx)) (.StamaniaCost (Utilities|Struct|BreakSt_MontageAction _returnvalue))))
    (:RowNotFound
      (return false 0 0.0))))