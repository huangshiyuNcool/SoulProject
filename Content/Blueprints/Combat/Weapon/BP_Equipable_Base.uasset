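; Base Blueprint for equipable items in the combat weapon system, tracking equipped state and attaching to the owning Character.
; OnEquipped sets the flag and snaps the item to AttachSocketName on the Character's mesh, while OnUnEquipped only clears the flag without detaching.
; GetItemMesh supports both mesh types, returning the static mesh component if it has a mesh assigned, otherwise the skeletal one.
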(event EventBeginPlay)

(event Collision|EventActorBeginOverlap
  (params (OtherActor :type Actor%20Object%20Reference)))

(event EventTick
  (params (DeltaSeconds :type Float%20%28single-precision%29)))

(fn ConstructionScript)

(fn GetItemMesh
  (Utilities|IsValid (Variables|/Script/Engine.StaticMeshComponent|GetStaticMesh (Variables|Default|GetStaticMesh))
    (:Is%20Valid
      (return (Variables|Default|GetStaticMesh)))
    (:Is%20Not%20Valid
      (return (Variables|Default|GetSkeletalMesh)))))

(fn OnEquipped
  (Variables|Default|SetbIsEquipped true)
  (ItemMesh|AttachActor (Variables|Default|GetAttach%20Socket%20Name)))

(fn OnUnEquipped
  (if (Variables|Default|GetbIsEquipped)
    (Variables|Default|SetbIsEquipped false)))

(fn SetIsEquipped
  (params (bIsEquipped :type Boolean))
  (Variables|Default|SetbIsEquipped bIsEquipped))

(fn AttachActor
  (params (SocketName :type Name))
  (Transformation|AttachComponentToComponent (Variables|/Script/Engine.Character|GetMesh (.AsCharacter (Utilities|Casting|CastToCharacter (Components|GetOwner)))) SocketName "SnapToTarget" "SnapToTarget" "SnapToTarget" true))

(fn GetIsEquipped
  (return (Variables|Default|GetbIsEquipped)))